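; BP_Coral_Force is a coral bubble vent that intermittently pushes the bubble player.
; From BeginPlay, it alternates between activating and deactivating its BubbleStream and Box components in an endless loop, with random delays of up to five seconds.
; When a BP_BubblePlayer begins overlapping the Box, a single AddForce call on its CharacterMovement pushes it along the actor's up vector, so rotation sets the push direction.
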(event `Activate Collision`
  (`ActorComponent.Activate` (`self.Bubble Stream`) false)
  (`ActorComponent.Activate` (`self.Box`) false)
  (`KismetSystemLibrary.Delay` (`KismetMathLibrary.RandomFloatInRange` 0.0 5.0))
  (`self.Deactivate Collision`))

(event `Deactivate Collision`
  (`ActorComponent.Deactivate` (`self.Bubble Stream`))
  (`ActorComponent.Deactivate` (`self.Box`))
  (`KismetSystemLibrary.Delay` (`KismetMathLibrary.RandomFloatInRange` 0.0 5.0))
  (`self.Activate Collision`))

(event `self.ReceiveBeginPlay`
  (`ActorComponent.Deactivate` (`self.Box`))
  (`KismetSystemLibrary.Delay` (`KismetMathLibrary.RandomFloatInRange` 0.0 5.0))
  (`self.Activate Collision`))

(event `self.Box.OnComponentBeginOverlap`
  (params (OverlappedComponent :type "PrimitiveComponent Object Reference") (OtherActor :type "Actor Object Reference") (OtherComp :type "PrimitiveComponent Object Reference") (OtherBodyIndex :type Integer) (bFromSweep :type Boolean) (SweepResult :type "HitResult Structure (by ref)"))
  (bind _asbp_bubble_player (cast `/Game/Player/BP_BubblePlayer` OtherActor))
  (`CharacterMovementComponent.AddForce` (`Character.CharacterMovement` _asbp_bubble_player) (* (`self.GetActorUpVector`) 500.0)))

(fn `UserConstructionScript`)