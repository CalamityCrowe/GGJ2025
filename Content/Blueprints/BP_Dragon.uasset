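; BP_Dragon is a dragon character that switches its Character Movement to Swimming mode on BeginPlay.
; Its construction script sets the mesh's skin and eye materials from two material arrays, indexed by the dragon's skin and eye index getters.
; GetForwardAimLocation is a stub that returns a zero vector.
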(event `self.ReceiveBeginPlay`
  (`CharacterMovementComponent.SetMovementMode` (`self.CharacterMovement`) "MOVE_Swimming" 0))

(fn `GetForwardAimLocation`
  (returns (FrontLocation :type "Vector Structure"))
  (return (0.0 0.0 0.0)))

(fn `UserConstructionScript`
  (locals (NewLocalVar :type "MaterialInterface Object Reference" :default "/Script/Engine.MaterialInstanceConstant'/Game/LittleDragons/Materials/Little_Dragon_Tiger/Realistic/MI_TD_Realistic_Black.MI_TD_Realistic_Black'"))
  (`PrimitiveComponent.SetMaterial` (`self.Mesh`) 0 (`|GetArrayItem` (`self.SkinMaterials`) (`self.GetDragonSkinIndex`)))
  (`PrimitiveComponent.SetMaterial` (`self.Mesh`) 1 (`|GetArrayItem` (`self.EyeMaterials`) (`self.GetDragonEyeIndex`))))