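; BP_BubblePlayer is the player's bubble character, handling swimming, HUD, trail effects, damage and death.
; A looping timer toggles the trail from velocity, and collecting randomly raises swim speed, grows the capsule through a timeline, or both.
; Damage bursts remove a HUD element, shake the camera and briefly disable input, with a separate timer restoring damageability.
; Death removes a HUD element, spawns a burst effect and destroys the actor.
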(event `Toggle Trail`
  (if (> (`KismetMathLibrary.VSizeSquared` (`self.GetVelocity`)) 0.0)
    (`self.Start Trail`)
    (else
      (`self.Stop Trail`))))

(event `self.ReceiveBeginPlay`
  (`KismetSystemLibrary.K2_SetTimerDelegate` (delegate `Toggle Trail`) 0.5 true)
  (bind _returnvalue (`|CreateWidget` "/Game/UI/WBP_HUD.WBP_HUD_C"))
  (bind _output_get (set `self.PlayerHud` _returnvalue))
  (`UserWidget.AddToViewport` _output_get 0))

(event `Start Trail`
  (`ActorComponent.Activate` (`self.Trail`) false)
  (`SceneComponent.SetVisibility` (`self.Trail`) true false))

(event `Start Swimming`
  ;[1 1 1] Handles the Swimming Stuff
  (bind _output_get (set `PhysicsVolume.bWaterVolume` true (`MovementComponent.GetPhysicsVolume` (`self.CharacterMovement`))))
  (set `self.IsSwimming` _output_get))

(event `Stop Trail`
  (`ActorComponent.Deactivate` (`self.Trail`))
  (`SceneComponent.SetVisibility` (`self.Trail`) true false))

(event `self.HandleDeath`
  (`/Game/UI/WBP_HUD.Remove Element` (`self.PlayerHud`))
  (`NiagaraFunctionLibrary.SpawnSystemAtLocation` "/Game/Niagara/NS_BubbleBurst.NS_BubbleBurst" (`self.K2_GetActorLocation`))
  (`self.K2_DestroyActor`))

(event `self.ActivateBurst`
  (`/Game/UI/WBP_HUD.Remove Element` (`self.PlayerHud`))
  (`self.DisableInput` (`GameplayStatics.GetPlayerController` 0))
  (`PlayerCameraManager.StartCameraShake` :`self` (`GameplayStatics.GetPlayerCameraManager` 0) :`ShakeClass` "/Game/Player/DamageShake.DamageShake_C" :`PlaySpace` "World")
  (`NiagaraFunctionLibrary.SpawnSystemAtLocation` "/Game/Niagara/NS_BurstDamage.NS_BurstDamage" (`self.K2_GetActorLocation`))
  (`Timeline|Delay Controller Activation` :!via `PlayFromStart`
    (:`Finished`
      (`self.EnableInput` (`GameplayStatics.GetPlayerController` 0)))))

(event `self.IFrames`
  (`Timeline|ResumeDamage` :!via `PlayFromStart`
    (:`Finished`
      (set `self.bCanDamage` true))))

(event `self.CollectReact`
  (bind _charactermovement (`self.CharacterMovement`))
  (bind _charactermovement_2 (`self.CharacterMovement`))
  (switch `int` (`KismetMathLibrary.RandomInteger` 3)
    (:`0`
      (set `CharacterMovementComponent.MaxSwimSpeed` (+ (`CharacterMovementComponent.MaxSwimSpeed` _charactermovement) 25.0) _charactermovement))
    (:`1`
      (set `self.Scale` (+ (`SceneComponent.K2_GetComponentScale` (`self.CapsuleComponent`)) (0.1 0.1 0.1)) :!label _label)
      (bind (_direction _newtrack_0) (`Timeline|Timeline` :!via `PlayFromStart`)
        (:`Update`
          (`SceneComponent.SetWorldScale3D` (`self.CapsuleComponent`) (`KismetMathLibrary.VLerp` (`self.GetActorRelativeScale3D`) (`self.Scale`) _newtrack_0)))))
    (:`2`
      (set `CharacterMovementComponent.MaxSwimSpeed` (+ (`CharacterMovementComponent.MaxSwimSpeed` _charactermovement_2) 25.0) _charactermovement_2)
      (goto _label))))

(fn `UserConstructionScript`)